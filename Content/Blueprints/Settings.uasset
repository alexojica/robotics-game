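; Trigger actor that opens the Settings menu and pauses the game when the player character enters its Box.
; On overlap it re-adds the first top-level Settings widget it finds, or creates one if none exists, then adds it to the viewport.
; A UI-only input mode call is present but unconnected, so the actor leaves input mode unchanged.
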(event OnComponentBeginOverlap(Box)
  (params (OverlappedComponent :type Primitive%20Component%20Object%20Reference) (OtherActor :type Actor%20Object%20Reference) (OtherComp :type Primitive%20Component%20Object%20Reference) (OtherBodyIndex :type Integer) (bFromSweep :type Boolean) (SweepResult :type Hit%20Result%20Structure%20%28by%20ref%29))
  (if (== OtherActor (Game|GetPlayerCharacter 0))
    (bind _foundwidgets (Widget|GetAllWidgetsOfClass "/Game/UI/Settings.Settings_C" true))
    (if (!= (Utilities|Array|Length _foundwidgets) 0)
      (UserInterface|Viewport|AddtoViewport (Utilities|Array|Get(acopy) _foundwidgets) 0)
      (else
        (bind _returnvalue (UserInterface|CreateWidget "/Game/UI/Settings.Settings_C"))
        (UserInterface|Viewport|AddtoViewport _returnvalue 0)))
    (Game|SetGamePaused true)))

(event EventBeginPlay)

(event Collision|EventActorBeginOverlap
  (params (OtherActor :type Actor%20Object%20Reference)))

(event EventTick
  (params (DeltaSeconds :type Float%20%28single-precision%29)))

(fn ConstructionScript)