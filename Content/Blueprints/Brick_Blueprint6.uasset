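; Brick actor that toggles its static mesh visibility based on what the player's Grabber component is hitting.
; Each Tick it compares the Grabber's hit actor on the ThirdPersonCharacter to itself by object name, and hides the mesh when they differ.
; The changemat event shows the mesh again, despite its name suggesting a material change.
; The material-swap nodes are left unconnected and never run.
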(event Custom|changemat
  (Rendering|SetVisibility (Variables|Debug|GetStaticMeshComponent) true false))

(event EventBeginPlay)

(event Collision|EventActorBeginOverlap
  (params (OtherActor :type Actor%20Object%20Reference)))

(event EventTick
  (params (DeltaSeconds :type Float%20%28single-precision%29))
  (if (not (Utilities|Enum|Equal(Enum) (Utilities|GetObjectName (.hitactor (Variables|/Script/Skystone_working.Grabber|GetObjectHit (Actor|GetComponentbyClass (.AsThird%20Person%20Character (Utilities|Casting|CastToThirdPersonCharacter (Game|GetPlayerCharacter 0))) "/Script/Skystone_working.Grabber")))) (Utilities|GetObjectName self)))
    (Rendering|SetVisibility (Variables|Debug|GetStaticMeshComponent) false false)))

(fn ConstructionScript)