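; Tutorial trigger actor that shows a Tutorial widget when the player character enters its Box.
; The overlap creates the widget and adds it to the viewport only if no top-level FirstTip or SecondTip widget exists.
; The Shown flag must be true to fire and is cleared after display, so the tutorial appears once, while a blocked overlap leaves it able to retry.
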(event OnComponentBeginOverlap(Box)
  (params (OverlappedComponent :type Primitive%20Component%20Object%20Reference) (OtherActor :type Actor%20Object%20Reference) (OtherComp :type Primitive%20Component%20Object%20Reference) (OtherBodyIndex :type Integer) (bFromSweep :type Boolean) (SweepResult :type Hit%20Result%20Structure%20%28by%20ref%29))
  (if (and (== OtherActor (Game|GetPlayerCharacter 0)) (Variables|Default|Getshown))
    (bind _foundwidgets (Widget|GetAllWidgetsOfClass "/Game/UI/Tips/FirstTip.FirstTip_C" true))
    (bind _foundwidgets_2 (Widget|GetAllWidgetsOfClass "/Game/UI/Tips/SecondTip.SecondTip_C" true))
    (if (not (or (!= (Utilities|Array|Length _foundwidgets_2) 0) (!= (Utilities|Array|Length _foundwidgets) 0)))
      (bind _returnvalue (UserInterface|CreateWidget "/Game/UI/tutorial.tutorial_C"))
      (UserInterface|Viewport|AddtoViewport _returnvalue 0)
      (Variables|Default|Setshown false))))

(event EventBeginPlay)

(event Collision|EventActorBeginOverlap
  (params (OtherActor :type Actor%20Object%20Reference)))

(event EventTick
  (params (DeltaSeconds :type Float%20%28single-precision%29)))

(fn ConstructionScript)