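; MyGameMode is a game mode that swaps player 0's pawn on BeginPlay for the character variant saved in the game instance.
; It destroys the current player character, loads the save through MyGameInstance and switches on its Robot value.
; That value picks ThirdPersonCharacter or ThirdPersonCharacter_Child, which is spawned at the player controller's transform and possessed.
; The PlayerStart lookup runs, but its result is unused.
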(event EventBeginPlay
  (bind _returnvalue (Game|GetGameInstance))
  (bind _returnvalue_2 (Game|GetPlayerController 0))
  (bind _returnvalue_3 (Game|GetPlayerController 0))
  (bind _returnvalue_4 (Transformation|GetActorTransform _returnvalue_3))
  (bind _asmy_game_instance (Utilities|Casting|CastToMyGameInstance _returnvalue))
  (bind _outactors (Actor|GetAllActorsOfClass "/Script/Engine.PlayerStart"))
  (Actor|DestroyActor (Game|GetPlayerCharacter 0))
  (Default|Load _asmy_game_instance)
  (switch int (Variables|/Game/Blueprints/SaveGameObj.SaveGameObj_C|Getrobot (Variables|/Game/Blueprints/MyGameInstance.MyGameInstance_C|GetSaveGameObject _asmy_game_instance))
    (:Default
      (bind _returnvalue_5 (Game|SpawnActorfromClass "/Game/ThirdPersonCPP/Blueprints/ThirdPersonCharacter.ThirdPersonCharacter_C" _returnvalue_4 "Undefined" 0 0.97 0 :!label _label))
      (Pawn|Possess _returnvalue_2 _returnvalue_5))
    (:0
      (goto _label))
    (:1
      (bind _returnvalue_6 (Game|SpawnActorfromClass "/Game/ThirdPersonCPP/Blueprints/ThirdPersonCharacter_Child.ThirdPersonCharacter_Child_C" _returnvalue_4 "Undefined" 0 0.15 0))
      (Pawn|Possess _returnvalue_2 _returnvalue_6))))

(event EventTick
  (params (DeltaSeconds :type Float%20%28single-precision%29)))

(fn ConstructionScript)