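; Bot AI logic that sends its controller toward the Brick_Blueprint actor nearest to player character 0.
; On BeginPlay, FindActorBP scans all bricks, keeps the closest by distance to the player rather than the bot, and starts a simple move to it.
; Tick reissues the move while that brick is valid; once it is invalid, it resets the stored minimum distance and position and searches again.
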(event Custom|FindActorBP
  (bind _outactors (Actor|GetAllActorsOfClass "/Game/Blueprints/Brick_Blueprint.Brick_Blueprint_C"))
  (for _array_element _outactors
    (if (< (Math|Vector|Distance(Vector) (.location (Transformation|GetActorTransform _array_element)) (.location (Transformation|GetActorTransform (Game|GetPlayerCharacter 0)))) (Variables|Default|Getmindist))
      (Variables|Default|Setmindist (Math|Vector|Distance(Vector) (.location (Transformation|GetActorTransform _array_element)) (.location (Transformation|GetActorTransform (Game|GetPlayerCharacter 0)))))
      (Variables|Default|Setpos (.location (Transformation|GetActorTransform _array_element)))
      (Variables|Default|SetBrick _array_element)))
  (AI|Navigation|SimpleMovetoActor self (Variables|Default|GetBrick)))

(event Custom|reset
  (Variables|Default|Setmindist 1e+10)
  (Variables|Default|Setpos "0, 0, 0"))

(event EventBeginPlay
  (CallFunction|FindActorBP))

(event Collision|EventActorBeginOverlap
  (params (OtherActor :type Actor%20Object%20Reference)))

(event EventTick
  (params (DeltaSeconds :type Float%20%28single-precision%29))
  (Utilities|IsValid (Variables|Default|GetBrick)
    (:Is%20Valid
      (AI|Navigation|SimpleMovetoActor self (Variables|Default|GetBrick)))
    (:Is%20Not%20Valid
      (CallFunction|Reset)
      (CallFunction|FindActorBP))))

(fn ConstructionScript)