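; Enemy AI character that gathers bricks and carries them to a drop location, starting six seconds after play begins.
; It finds the nearest brick by distance, walks to it with simple move nodes, then swaps it for a collisionless copy attached to a hand socket.
; At the drop point it destroys the copy and spawns a placed brick at a set location, using timed boolean flags to mark grab and place phases.
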(event Custom|FindActorBP
  (bind _outactors (Actor|GetAllActorsOfClass (Variables|Default|GetBrickClass2)))
  (for _array_element _outactors
    (if (< (Math|Vector|Distance(Vector) (.location (Transformation|GetActorTransform _array_element)) (.location (Transformation|GetActorTransform))) (Variables|Default|Getmindist))
      (Variables|Default|Setmindist (Math|Vector|Distance(Vector) (.location (Transformation|GetActorTransform _array_element)) (.location (Transformation|GetActorTransform))))
      (Variables|Default|SetBrick _array_element))))

(event Custom|reset
  (Variables|Default|Setmindist 1e+10))

(event Custom|pick_up_stone
  (params (NewParam :type Vector))
  (Variables|Default|Setcan false)
  (Variables|Default|Setgheara true)
  (Variables|Default|Setprindere true)
  (Utilities|FlowControl|Delay 0.96)
  (Variables|Default|Setprindere false)
  (Utilities|FlowControl|Delay 0.15)
  (Variables|Default|Setgheara false)
  (Variables|Default|SetFull true)
  (Actor|DestroyActor (Variables|Default|GetBrick))
  (Variables|Default|Setcan true)
  (bind _returnvalue (Game|SpawnActorfromClass "/Game/Blueprints/Brick_Blueprint3.Brick_Blueprint3_C" (Math|Transform|MakeTransform (Math|Random|RandomUnitVector) "0, 0, 0" "1,1,1") "Undefined" 0 0))
  (Collision|SetCollisionEnabled (Variables|/Script/Engine.StaticMeshActor|GetStaticMeshComponent _returnvalue) "NoCollision")
  (Transformation|AttachComponentToComponent (Variables|/Script/Engine.StaticMeshActor|GetStaticMeshComponent _returnvalue) (Variables|Character|GetMesh) "PrindereSocket" "SnapToTarget" "SnapToTarget" "KeepWorld" true)
  (Utilities|FlowControl|Delay 0.4)
  (Variables|Default|Setprindere2 false)
  (AI|Navigation|SimpleMovetoLocation (Pawn|GetController self) (Variables|Default|GetLoc)))

(event EventBeginPlay
  (Utilities|FlowControl|Delay 6.0)
  (CallFunction|FindActorBP)
  (Variables|Default|SetCanplay true)
  (Variables|Default|SetCustomTimeDilation 0.5))

(event EventTick
  (params (DeltaSeconds :type Float%20%28single-precision%29))
  (bind _self self)
  (bind _loc (Variables|Default|GetLoc))
  (bind _returnvalue (Transformation|GetActorLocation _self))
  (Variables|Default|Setforward (Input|AxisValues|GetMoveForward))
  (Variables|Default|Setright (Input|AxisValues|GetMoveRight))
  (if (Variables|Default|GetCanplay)
    (Utilities|FlowControl|Delay 1.0)
    (Utilities|IsValid (Variables|Default|GetBrick)
      (:Is%20Valid
        (if (Variables|Default|Getcan)
          (if (< (Math|Vector|Distance(Vector) (Transformation|GetActorLocation (Variables|Default|GetBrick)) _returnvalue) 1.3e+02)
            (CallFunction|PickUpStone "0, 0, 0")
            (else
              (AI|Navigation|SimpleMovetoActor (Pawn|GetController self) (Variables|Default|GetBrick))))))
      (:Is%20Not%20Valid
        (if (Variables|Default|GetFull)
          (if (Math|Vector|Equal(Vector) _returnvalue (Variables|Default|GetLoc) 1e+02)
            (Variables|Default|Setgheara true)
            (Utilities|FlowControl|Delay 0.15)
            (Variables|Default|Setgheara false)
            (Actor|DestroyActor (stale Custom|pick_up_stone _returnvalue))
            (bind _returnvalue_2 (Game|SpawnActorfromClass (Variables|Default|GetBrickClass) (Math|Transform|MakeTransform (Variables|Default|GetSpawnLoc) "0, 0, 0" "1,1,1") "Undefined" 0 0))
            (Variables|Default|SetFull false)
            (Variables|/Script/Engine.PrimitiveComponent|SetCanCharacterStepUpOn (Actor|GetComponentbyClass _returnvalue_2 "/Script/Engine.StaticMeshComponent") "ECB_No")
            (Utilities|FlowControl|Delay 0.76)
            (Variables|Default|Setpunere2 true)
            (Utilities|FlowControl|Delay 0.2)
            (Variables|Default|Setpunere2 false)
            (else
              (AI|Navigation|SimpleMovetoLocation (Pawn|GetController self) (Math|Vector|MakeVector (.x _loc) (.y _loc) (.z _loc)))))
          (else
            (CallFunction|Reset)
            (CallFunction|FindActorBP)))))))

(fn ConstructionScript)